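; Grass is a cuttable grass actor that the truck character cuts by driving into it.
; When the truck's capsule overlaps its collision, a DoOnce gate runs Cut a single time.
; Cut spawns a particle burst, sets a "Cut" parameter on a dynamic material instance, plays controller force feedback and reports the consumed grass to GM_Main.
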(event `self.Collision.OnComponentBeginOverlap`
  (params (OverlappedComponent :type "PrimitiveComponent Object Reference") (OtherActor :type "Actor Object Reference") (OtherComp :type "PrimitiveComponent Object Reference") (OtherBodyIndex :type Integer) (bFromSweep :type Boolean) (SweepResult :type "HitResult Structure (by ref)"))
  (bind _astruck_character_1 (cast `/Game/PlayerCharacter/TruckCharacter1` OtherActor))
  (if (== OtherComp (`Character.CapsuleComponent` _astruck_character_1))
    (`/Engine/EditorBlueprintResources/StandardMacros.DoOnce` false
      (:`Completed`
        (`self.Cut`)))))

(fn `Cut`
  (`GameplayStatics.SpawnEmitterAtLocation` "/Game/Enrivonment/Grass/PS_Grass_Cut_01.PS_Grass_Cut_01" (`self.K2_GetActorLocation`))
  (bind _returnvalue (`PrimitiveComponent.CreateDynamicMaterialInstance` (`self.Grass`) 0 null "None"))
  (`MaterialInstanceDynamic.SetScalarParameterValue` _returnvalue "Cut" 1.0)
  (`PlayerController.K2_ClientPlayForceFeedback` (`GameplayStatics.GetPlayerController` 0) "/Game/Feedback/FF_Cut.FF_Cut" "None" false false false)
  (bind _asgm_main (cast `/Game/Core/GM_Main` (`GameplayStatics.GetGameMode`)))
  (`/Game/Core/GM_Main.GrassConsumed` _asgm_main))

(fn `UserConstructionScript`)