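; PC_Main is the player controller that drives TruckCharacter1 and handles restart and quit input.
; During one GM_Main state, Gas pushes the truck forward with a minimum throttle, stores the throttle and scales its fire components.
; Steering adds yaw scaled by delta time, rotation rate and a curve of current throttle.
; Start reloads the level in two other states, Exit quits anytime, and MoveForward plus older rotation experiments are unused.
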(event `InputAxis|MoveForward`
  (params (AxisValue :type "Float (single-precision)"))
  ;[1 0 0] Currently Not Used
)

(event `InputAxis|MoveRight`
  (params (AxisValue :type "Float (single-precision)"))
  ;[1 1 1] Rotation of Truck
  (bind _asgm_main (cast `/Game/Core/GM_Main` (`GameplayStatics.GetGameMode`)))
  (if (`|EnumEquality` (`/Game/Core/GM_Main.State` _asgm_main) "NewEnumerator2")
    (bind _astruck_character_1 (cast `/Game/PlayerCharacter/TruckCharacter1` (`self.K2_GetPawn`)))
    (`Pawn.AddControllerYawInput` _astruck_character_1 (* AxisValue (`self.RotationRate`) (`GameplayStatics.GetWorldDeltaSeconds`) (`CurveFloat.GetFloatValue` (`self.RotationRateCurve`) (`KismetMathLibrary.FClamp` (`self.GetInputAxisValue`) (`self.MinimumThrottle`)))))))

(event `InputAxis|Gas`
  (params (AxisValue :type "Float (single-precision)"))
  (bind _returnvalue (`self.K2_GetPawn`))
  (bind _returnvalue_2 (`KismetMathLibrary.FClamp` AxisValue (`self.MinimumThrottle`)))
  ;[1 1 1] Throttling
  (bind _asgm_main (cast `/Game/Core/GM_Main` (`GameplayStatics.GetGameMode`)))
  (if (`|EnumEquality` (`/Game/Core/GM_Main.State` _asgm_main) "NewEnumerator2")
    (bind _astruck_character_1 (cast `/Game/PlayerCharacter/TruckCharacter1` _returnvalue))
    (`Pawn.AddMovementInput` _astruck_character_1 (`self.GetActorForwardVector` _returnvalue) _returnvalue_2 false)
    (set `/Game/PlayerCharacter/TruckCharacter1.Throttle` _returnvalue_2 _astruck_character_1)
    (for _array_element (`/Game/PlayerCharacter/TruckCharacter1.Get Fires` _astruck_character_1)
      (`SceneComponent.SetRelativeScale3D` _array_element (`KismetMathLibrary.Conv_DoubleToVector` AxisValue)))))

(event `InputAction|Start`
  (params (Key :type "Key Structure"))
  (:`Pressed`
    (bind _asgm_main (cast `/Game/Core/GM_Main` (`GameplayStatics.GetGameMode`)))
    (bind _state (`/Game/Core/GM_Main.State` _asgm_main))
    (if (or (`|EnumEquality` _state "NewEnumerator3") (`|EnumEquality` _state "NewEnumerator5"))
      (bind _returnvalue (`GameplayStatics.GetCurrentLevelName` true))
      (`GameplayStatics.OpenLevel` (`KismetStringLibrary.Conv_StringToName` _returnvalue)))))

(event `InputAction|Exit`
  (params (Key :type "Key Structure"))
  (:`Pressed`
    (`KismetSystemLibrary.QuitGame` null "Quit")))

(fn `UserConstructionScript`)