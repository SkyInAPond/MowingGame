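; Game mode that runs a truck grass-eating game, where gas is the timer and clearing all Grass actors wins.
; BeginPlay creates the main HUD, counts the grass and sets the game active after a one-second delay.
; While active and not in debug, Tick drains and prints gas, failing once when empty.
; GrassConsumed refills gas and decrements the count; win and fail update both HUD and state.
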(event `self.ReceiveBeginPlay`
  (`|ExecutionSequence`
    (:`then_0`
      (bind _returnvalue (`|CreateWidget` "/Game/UI/UI_Main.UI_Main_C"))
      (`UserWidget.AddToViewport` _returnvalue 0)
      (set `self.Main HUD` _returnvalue)
      (`KismetSystemLibrary.Delay` 1.0)
      (bind _astruck_character_1 (cast `/Game/PlayerCharacter/TruckCharacter1` (`GameplayStatics.GetPlayerPawn` 0)))
      (set `self.PreviousLocation` (`self.K2_GetActorLocation` _astruck_character_1))
      (set `self.State` "NewEnumerator2"))
    (:`then_1`
      (bind _outactors (`GameplayStatics.GetAllActorsOfClass` "/Game/Blueprints/Grass.Grass_C"))
      (bind _output_get (set `self.GrassLeft` (`KismetArrayLibrary.Array_Length` _outactors)))
      (set `self.InitialGrass` _output_get))))

(event `Fail`
  (params (Reason :type "/Game/Core/GameStates Enum" :default "NewEnumerator0"))
  (`/Engine/EditorBlueprintResources/StandardMacros.DoOnce` false
    (:`Completed`
      (`/Game/UI/UI_Main.Fail` (`self.Main HUD`) Reason)
      (set `self.State` Reason))))

(event `self.ReceiveTick`
  (params (DeltaSeconds :type "Float (single-precision)"))
  (switch `/Game/Core/GameStates` (`self.State`)
    (:`NewEnumerator2`
      (if (not (`self.Debug`))
        (bind _astruck_character_1 (cast `/Game/PlayerCharacter/TruckCharacter1` (`GameplayStatics.GetPlayerPawn` 0)))
        (bind _output_get (set `self.GasLeft` (- (`self.GasLeft`) (* (`self.GasDecreasePerSecond`) (`GameplayStatics.GetWorldDeltaSeconds`)))))
        (set `self.PreviousLocation` (`self.K2_GetActorLocation` _astruck_character_1))
        (`KismetSystemLibrary.PrintString` (`KismetStringLibrary.Concat_StrStr` "Gas Left: " (`KismetStringLibrary.Conv_DoubleToString` (`self.GasLeft`))) true true (struct :`G` 0.66 :`B` 1.0 :`A` 1.0) 0.0)
        (`/Engine/EditorBlueprintResources/StandardMacros.CompareFloat` _output_get
          (:`<`
            (`self.Fail` "NewEnumerator3")))))))

(event `GrassConsumed`
  (set `self.GasLeft` (+ (`self.GasLeft`) (`self.GasIncreasePerGrass`)))
  (bind _result (`/Engine/EditorBlueprintResources/StandardMacros.DecrementInt` (`self.GrassLeft`))
    (:`  `
      (`/Engine/EditorBlueprintResources/StandardMacros.CompareInt` _result
        (:`==`
          _)
        (:`<`
          _))
      (`self.Win`))))

(event `Win`
  (`/Game/UI/UI_Main.Win` (`self.Main HUD`))
  (set `self.State` "NewEnumerator4"))

(fn `UserConstructionScript`)